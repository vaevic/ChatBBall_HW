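; BP_Controller is a controller that links the WBP_ChatWindow widget to BP_ChatMode for networked chat with user IDs.
; After a short BeginPlay delay, it binds an event to the chat window's message delegate.
; Outgoing messages go raw to the game mode, then slash-prefixed ones reach ServerProcessChatMessage while others are resent with the user ID prepended.
; Other events store the login ID, print broadcasts on authority and append received messages to the chat log.
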(event Custom|OnsendMsgToServer
  (params (msg :type String))
  (bind _asbp_chat_mode (Utilities|Casting|CastToBP_ChatMode (Game|GetGameMode)))
  (Default|GotMessagefromClient _asbp_chat_mode msg)
  (if (Utilities|String|StartsWith msg "/")
    (Development|PrintString msg true true "(R=0.407385,G=0.054203,B=1.000000,A=1.000000)")
    (Class|NumBaseballGamePlayerController|ServerProcessChatMessage msg)
    (else
      (Default|GotMessagefromClient _asbp_chat_mode (Utilities|String|Append (Variables|Default|GetUserID) ":" msg)))))

(event Custom|GotBroadcast
  (params (msg :type String))
  (if (Ability|HasAuthority)
    (Development|PrintString msg true true "(R=0.000000,G=0.660000,B=1.000000,A=1.000000)" 1e+01)))

(event Custom|OnLoginWithID
  (params (User%20ID :type String))
  (Default|CallOnUserLogin User%20ID)
  (Variables|Default|SetUserID User%20ID))

(event EventBeginPlay
  (if (not (Utilities|Enum|Equal(Enum) (Class|Actor|GetRemoteRole) "ROLE_None"))
    (Utilities|FlowControl|Delay 0.2)
    (bind _foundwidgets (Widget|GetAllWidgetsOfClass "/Game/Widget/WBP_ChatWindow.WBP_ChatWindow_C" true))
    (bind _output_get (Variables|Default|SetWidget (Utilities|Array|Get(acopy) _foundwidgets)))
    (bind _aswbp_chat_window (Utilities|Casting|CastToWBP_ChatWindow _output_get))
    (EventDispatchers|BindEventtoSetMessagetoUserController _aswbp_chat_window (EventDispatchers|CreateEvent :!event Custom|OnsendMsgToServer))))

(event EventOnDisplayMessage
  (params (Message :type String))
  (bind _foundwidgets (Widget|GetAllWidgetsOfClass "/Game/Widget/WBP_ChatWindow.WBP_ChatWindow_C" false))
  (Development|PrintString Message true true "(R=1.000000,G=0.000000,B=0.463968,A=1.000000)")
  (Default|AddChatMessagetoLog (Utilities|Array|Get(acopy) _foundwidgets) Message))

(fn ConstructionScript)