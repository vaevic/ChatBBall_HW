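; BP_ChatMode is a game mode that gates game start on player count and relays chat messages between players.
; On each login it checks the GameState player array, calling StartNewGame once at least two players are present and printing a ready message otherwise.
; GotMessageFromClient acts as the broadcast hub, passing a message to every BP_Controller through GotBroadcast.
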(event Custom|GotMessageFromClient
  (params (Msg :type String))
  (bind _outactors (Actor|GetAllActorsOfClass "/Game/Blueprint/BP_Controller.BP_Controller_C"))
  (for _array_element _outactors
    (bind _asbp_controller (Utilities|Casting|CastToBP_Controller _array_element))
    (Default|GotBroadcast _asbp_controller Msg)))

(event EventBeginPlay)

(event EventTick
  (params (DeltaSeconds :type Float%20%28single-precision%29)))

(event EventPostLogin
  (params (NewPlayer :type Player%20Controller%20Object%20Reference))
  (bind _returnvalue (Game|GetGameState))
  (Utilities|Casting|CastToGameState _returnvalue)
  (if (>= (Utilities|Array|Length (Variables|/Script/Engine.GameStateBase|GetPlayerArray _returnvalue)) 2)
    (Class|NumBaseballGameMode|StartNewGame)
    (else
      (Development|PrintString "ready"))))

(fn ConstructionScript)